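; Destructible hanging-ice actor whose pieces fracture from damage when they register a hit.
; Hit events on three hanging-ice destructible mesh components each apply a small, full-strength radius damage to that same component at the impact point.
; The cube component's hit event is empty, and a directional damage call and an extra radius damage call are left unconnected.
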(event `self.1M_Cube_DM.OnComponentHit`
  (params (HitComponent :type "PrimitiveComponent Object Reference") (OtherActor :type "Actor Object Reference") (OtherComp :type "PrimitiveComponent Object Reference") (NormalImpulse :type "Vector Structure") (Hit :type "HitResult Structure (by ref)")))

(event `self.SM_HangingIce04_DM.OnComponentHit`
  (params (HitComponent :type "PrimitiveComponent Object Reference") (OtherActor :type "Actor Object Reference") (OtherComp :type "PrimitiveComponent Object Reference") (NormalImpulse :type "Vector Structure") (Hit :type "HitResult Structure (by ref)"))
  (`DestructibleComponent.ApplyRadiusDamage` (`self.SM_HangingIce04_DM`) 15.0 (`.Location` (`GameplayStatics.BreakHitResult` Hit)) 40.0 0.0 true))

(event `self.SM_HangingIce03_DM.OnComponentHit`
  (params (HitComponent :type "PrimitiveComponent Object Reference") (OtherActor :type "Actor Object Reference") (OtherComp :type "PrimitiveComponent Object Reference") (NormalImpulse :type "Vector Structure") (Hit :type "HitResult Structure (by ref)"))
  (`DestructibleComponent.ApplyRadiusDamage` (`self.SM_HangingIce03_DM`) 15.0 (`.Location` (`GameplayStatics.BreakHitResult` Hit)) 40.0 0.0 true))

(event `self.SM_HangingIce02_DM.OnComponentHit`
  (params (HitComponent :type "PrimitiveComponent Object Reference") (OtherActor :type "Actor Object Reference") (OtherComp :type "PrimitiveComponent Object Reference") (NormalImpulse :type "Vector Structure") (Hit :type "HitResult Structure (by ref)"))
  (`DestructibleComponent.ApplyRadiusDamage` (`self.SM_HangingIce02_DM`) 15.0 (`.Location` (`GameplayStatics.BreakHitResult` Hit)) 40.0 0.0 true))

(fn `UserConstructionScript`)